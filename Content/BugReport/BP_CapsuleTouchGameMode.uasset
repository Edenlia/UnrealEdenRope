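; Game mode in a BugReport folder that chains a registered character to a physics-simulated rigid rope.
; Registering a character stores it and spawns a replicated EdenRigidRopeActor at its ConstraintNode, using the ERR_Sausage rope asset.
; A spawned PhysicsConstraintActor then links the character's capsule to the rope's first particle, addressed as a bone.
; Physics replication to the autonomous proxy is turned off on the rope component.
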(event `RegisterChainedCharacter`
  (params (Character :type "/Game/BugReport/BP_CapsuleTouchCharacter Object Reference"))
  (set `self.Character0` Character)
  (`self.StartChain`))

(event `StartChain`
  (bind _returnvalue (`|SpawnActorFromClass` "/Script/EdenRope.EdenRigidRopeActor" (`KismetMathLibrary.Conv_VectorToTransform` (`SceneComponent.K2_GetComponentLocation` (`/Game/BugReport/BP_CapsuleTouchCharacter.ConstraintNode` (`self.Character0`)))) "Undefined" "MultiplyWithRoot" null null))
  (`self.SetReplicates` _returnvalue true)
  (`self.SetReplicateMovement` _returnvalue true)
  (bind _ropecomponent (`EdenRigidRopeActor.RopeComponent` _returnvalue))
  (`ActorComponent.SetIsReplicated` _ropecomponent true)
  (set `PrimitiveComponent.bReplicatePhysicsToAutonomousProxy` false _ropecomponent)
  (`EdenRigidRopeComponent.SetRopeAsset` _ropecomponent "/EdenRope/RigidRope/Asset/ERR_Sausage.ERR_Sausage")
  (`PrimitiveComponent.SetSimulatePhysics` _ropecomponent true)
  (set `self.Rope Component_0` _ropecomponent)
  (bind _returnvalue_2 (`|SpawnActorFromClass` "/Script/Engine.PhysicsConstraintActor" (`KismetMathLibrary.Conv_VectorToTransform` (`SceneComponent.K2_GetComponentLocation` (`/Game/BugReport/BP_CapsuleTouchCharacter.ConstraintNode` (`self.Character0`)))) "Undefined" "MultiplyWithRoot" null null))
  (bind _output_get (set `self.Constraint Comp` (`PhysicsConstraintActor.ConstraintComp` _returnvalue_2)))
  (`PhysicsConstraintComponent.SetConstrainedComponents` _output_get (`Character.CapsuleComponent` (`self.Character0`)) "None" (`self.Rope Component_0`) "Particle_0"))

(fn `UserConstructionScript`)