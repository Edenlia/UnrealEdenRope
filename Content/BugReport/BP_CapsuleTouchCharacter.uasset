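; BP_CapsuleTouchCharacter is a player-controllable character in the BugReport folder that registers with BP_CapsuleTouchGameMode as a chained character.
; On BeginPlay it adds the IMC_ChainedMan Enhanced Input context to player controller 0, then passes itself to the game mode.
; IA_Move drives movement relative to that controller's yaw, and IA_Look feeds controller yaw and pitch.
; The chain and capsule-touch behavior is not implemented in these graphs.
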(event `self.ReceiveBeginPlay`
  (`EnhancedInputSubsystemInterface.AddMappingContext` (pcsubsystem `EnhancedInputLocalPlayerSubsystem` (`GameplayStatics.GetPlayerController` 0)) "/EdenRope/Demo_Rigid/ChainedMan/Input/IMC_ChainedMan.IMC_ChainedMan" 0 (struct))
  (bind _asbp_capsule_touch_game_mode (cast `/Game/BugReport/BP_CapsuleTouchGameMode` (`GameplayStatics.GetGameMode`)))
  (`/Game/BugReport/BP_CapsuleTouchGameMode.RegisterChainedCharacter` _asbp_capsule_touch_game_mode self))

(event `EnhancedInput|/EdenRope/Demo_Rigid/ChainedMan/Input/IA_Move`
  (params (ActionValue :type "Vector2D Structure") (ElapsedSeconds :type "Float (double-precision)") (TriggeredSeconds :type "Float (double-precision)") (InputAction :type "InputAction Object Reference" :default "/EdenRope/Demo_Rigid/ChainedMan/Input/IA_Move.IA_Move"))
  (bind (_x _y) (`KismetMathLibrary.BreakVector2D` ActionValue))
  (bind (_returnvalue_roll _returnvalue_pitch _returnvalue_yaw) (`KismetMathLibrary.BreakRotator` (`Controller.GetControlRotation` (`GameplayStatics.GetPlayerController` 0))))
  (bind _returnvalue (`KismetMathLibrary.MakeRotator` 0.0 0.0 _returnvalue_yaw))
  (:`Triggered`
    (`self.AddMovementInput` (`KismetMathLibrary.GetForwardVector` _returnvalue) _y)
    (`self.AddMovementInput` (`KismetMathLibrary.GetRightVector` _returnvalue) _x)))

(event `EnhancedInput|/EdenRope/Demo_Rigid/ChainedMan/Input/IA_Look`
  (params (ActionValue :type "Vector2D Structure") (ElapsedSeconds :type "Float (double-precision)") (TriggeredSeconds :type "Float (double-precision)") (InputAction :type "InputAction Object Reference" :default "/EdenRope/Demo_Rigid/ChainedMan/Input/IA_Look.IA_Look"))
  (bind (_x _y) (`KismetMathLibrary.BreakVector2D` ActionValue))
  (:`Triggered`
    (`self.AddControllerYawInput` _x)
    (`self.AddControllerPitchInput` _y)))

(fn `UserConstructionScript`)